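; BP_EnemyAI is an enemy pawn that chases the player once it sees a pawn or hears a noise.
; PawnSensing events set CanSeePlayer and call FollowPlayer, which uses AI MoveTo toward player 0's character, whoever triggered the sense.
; Hearing also prints the instigator's name.
; CanSeePlayer is never cleared after detection, as the only reset sits in the branch where it is already false.
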(event OnSeePawn(PawnSensing)
  (params (Pawn :type Pawn%20Object%20Reference))
  (Variables|Default|SetcanSeePlayer true)
  (CallFunction|FollowPlayer))

(event OnHearNoise(PawnSensing)
  (params (Instigator :type Pawn%20Object%20Reference) (Location :type Vector%20%28by%20ref%29 :default "0, 0, 0") (Volume :type Float%20%28single-precision%29))
  (Development|PrintString (Utilities|GetDisplayName Instigator))
  (Variables|Default|SetcanSeePlayer true)
  (CallFunction|FollowPlayer))

(event Custom|FollowPlayer
  (if (Variables|Default|GetcanSeePlayer)
    (AI|AIMoveTo self "0, 0, 0" (Game|GetPlayerCharacter 0) 7e+01 false)
    (else
      (Variables|Default|SetcanSeePlayer false))))

(event EventBeginPlay)

(event Collision|EventActorBeginOverlap
  (params (OtherActor :type Actor%20Object%20Reference)))

(event EventTick
  (params (DeltaSeconds :type Float%20%28single-precision%29)))

(fn ConstructionScript)